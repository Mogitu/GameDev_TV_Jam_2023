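; Monster enemy character that attacks the player, handles catching them at zero health, and plays its own death sequence.
; A looping timer reads the AI blackboard's CanSeePlayer key and checks distance to set Attacking.
; Hand collider overlaps deal damage gated by Hittable; a killing hit stops movement, turns the monster via timeline and flags the player Caught.
; MonsterDies stops morph-target blinking, disables collision and movement, then spawns delayed ember and fire effects.
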(event OnComponentBeginOverlap(CollisionSphere)
  (params (OverlappedComponent :type Primitive%20Component%20Object%20Reference) (OtherActor :type Actor%20Object%20Reference) (OtherComp :type Primitive%20Component%20Object%20Reference) (OtherBodyIndex :type Integer) (bFromSweep :type Boolean) (SweepResult :type Hit%20Result%20Structure%20%28by%20ref%29))
  ;[1 1 1] PlayerDeath
)

(event OnComponentBeginOverlap(AttackColliderR)
  (params (OverlappedComponent :type Primitive%20Component%20Object%20Reference) (OtherActor :type Actor%20Object%20Reference) (OtherComp :type Primitive%20Component%20Object%20Reference) (OtherBodyIndex :type Integer) (bFromSweep :type Boolean) (SweepResult :type Hit%20Result%20Structure%20%28by%20ref%29))
  ;[1 1 1] HitPlayer
  (if (== (Utilities|Array|Get(acopy) (Variables|/Script/Engine.Actor|GetTags OtherActor)) "Player")
    (if (Variables|Default|GetHittable?)
      (Class|GJGameplayFunctionLibrary|DamageActor self (stale EventBeginPlay _asbp_player_character) 25.0)
      (Audio|PlaySound2D "/Game/_Game/Audio/Player_Hurt.Player_Hurt" (Math|Random|RandomFloatinRange 0.9 1.1) (Math|Random|RandomFloatinRange 0.7 1.2) 0.0 0 0 false)
      (Game|Feedback|ClientStartCameraShake (Pawn|GetLocalViewingPlayerController (Variables|Default|GetPlayer)) "/Game/_Game/Characters/CS_GetHit.CS_GetHit_C" 5e+01 "CameraLocal" "0, 0, 0")
      (bind _returnvalue (Class|GJHealthComponent|GetHealthComponent (Variables|Default|GetPlayer)))
      (if (<= (Class|GJHealthComponent|GetHealthFraction _returnvalue) 0.0)
        ;[1 1 1] PlayerDeath
        (Utilities|FlowControl|DoOnce false
          (:Completed
            (Variables|Default|SetAttacking false)
            (Variables|Default|SetHittable? false)
            (Variables|Default|SetPlayerCaught true)
            (Pawn|Components|CharacterMovement|SetMovementMode (Variables|Character|GetCharacterMovement) "MOVE_None" 0)
            (bind _newtrack_0 (Timeline|RotateToPlayer PlayFromStart)
              (:Update
                (Transformation|SetWorldRotation (Variables|Default|GetCapsuleComponent) (Math|Interpolation|RInterpTo (Math|Rotator|MakeRotator 0.0 0.0 (.yaw (Transformation|GetWorldRotation (Variables|Default|GetCapsuleComponent)))) (Math|Rotator|MakeRotator 0.0 0.0 (.yaw (Math|Rotator|FindLookatRotation (Transformation|GetWorldLocation (Variables|Default|GetCapsuleComponent)) (Transformation|GetWorldLocation (Variables|/Script/Engine.Character|GetMesh (Game|GetPlayerCharacter 0)))))) _newtrack_0 0.2) false false)
                (bind _asbp_player_character (Utilities|Casting|CastToBP_PlayerCharacter (Game|GetPlayerCharacter 0)))
                (Variables|/Game/_Game/Characters/BP_PlayerCharacter.BP_PlayerCharacter_C|SetCaught _asbp_player_character true)
                (Variables|/Game/_Game/Characters/BP_PlayerCharacter.BP_PlayerCharacter_C|SetMonster _asbp_player_character self)
                (if (Variables|Default|GetMonsterDead?)
                  (Variables|/Game/_Game/Characters/BP_PlayerCharacter.BP_PlayerCharacter_C|SetCaught _asbp_player_character false))))))
        (else
          (Variables|Default|SetHittable? false)
          (Effects|SpawnEmitteratLocation "/Game/Realistic_Starter_VFX_Pack_Vol2/Particles/Blood/P_Blood_Splat_Cone.P_Blood_Splat_Cone" (Transformation|GetWorldLocation (Variables|/Script/Engine.Actor|GetRootComponent (Variables|Default|GetPlayer))) "0, 0, 0" "50.000000,50.000000,50.000000"))))))

(event OnComponentBeginOverlap(AttackColliderL)
  (params (OverlappedComponent :type Primitive%20Component%20Object%20Reference) (OtherActor :type Actor%20Object%20Reference) (OtherComp :type Primitive%20Component%20Object%20Reference) (OtherBodyIndex :type Integer) (bFromSweep :type Boolean) (SweepResult :type Hit%20Result%20Structure%20%28by%20ref%29))
  ;[1 1 1] HitPlayer
  (if (== (Utilities|Array|Get(acopy) (Variables|/Script/Engine.Actor|GetTags OtherActor)) "Player")
    (if (Variables|Default|GetHittable?)
      (Class|GJGameplayFunctionLibrary|DamageActor self (stale EventBeginPlay _asbp_player_character) 25.0)
      (Audio|PlaySound2D "/Game/_Game/Audio/Player_Hurt.Player_Hurt" (Math|Random|RandomFloatinRange 0.9 1.1) (Math|Random|RandomFloatinRange 0.7 1.2) 0.0 0 0 false)
      (Game|Feedback|ClientStartCameraShake (Pawn|GetLocalViewingPlayerController (Variables|Default|GetPlayer)) "/Game/_Game/Characters/CS_GetHit.CS_GetHit_C" 5e+01 "CameraLocal" "0, 0, 0")
      (bind _returnvalue (Class|GJHealthComponent|GetHealthComponent (Variables|Default|GetPlayer)))
      (if (<= (Class|GJHealthComponent|GetHealthFraction _returnvalue) 0.0)
        ;[1 1 1] PlayerDeath
        (Utilities|FlowControl|DoOnce false
          (:Completed
            (Variables|Default|SetAttacking false)
            (Variables|Default|SetHittable? false)
            (Variables|Default|SetPlayerCaught true)
            (Pawn|Components|CharacterMovement|SetMovementMode (Variables|Character|GetCharacterMovement) "MOVE_None" 0)
            (bind _newtrack_0 (Timeline|RotateToPlayer PlayFromStart)
              (:Update
                (Transformation|SetWorldRotation (Variables|Default|GetCapsuleComponent) (Math|Interpolation|RInterpTo (Math|Rotator|MakeRotator 0.0 0.0 (.yaw (Transformation|GetWorldRotation (Variables|Default|GetCapsuleComponent)))) (Math|Rotator|MakeRotator 0.0 0.0 (.yaw (Math|Rotator|FindLookatRotation (Transformation|GetWorldLocation (Variables|Default|GetCapsuleComponent)) (Transformation|GetWorldLocation (Variables|/Script/Engine.Character|GetMesh (Game|GetPlayerCharacter 0)))))) _newtrack_0 0.2) false false)
                (bind _asbp_player_character (Utilities|Casting|CastToBP_PlayerCharacter (Game|GetPlayerCharacter 0)))
                (Variables|/Game/_Game/Characters/BP_PlayerCharacter.BP_PlayerCharacter_C|SetCaught _asbp_player_character true)
                (Variables|/Game/_Game/Characters/BP_PlayerCharacter.BP_PlayerCharacter_C|SetMonster _asbp_player_character self)
                (if (Variables|Default|GetMonsterDead?)
                  (Variables|/Game/_Game/Characters/BP_PlayerCharacter.BP_PlayerCharacter_C|SetCaught _asbp_player_character false))))))
        (else
          (Variables|Default|SetHittable? false)
          (Effects|SpawnEmitteratLocation "/Game/Realistic_Starter_VFX_Pack_Vol2/Particles/Blood/P_Blood_Splat_Cone.P_Blood_Splat_Cone" (Transformation|GetWorldLocation (Variables|/Script/Engine.Actor|GetRootComponent (Variables|Default|GetPlayer))) "0, 0, 0" "50.000000,50.000000,50.000000"))))))

(event Custom|MonsterDies
  (bind _returnvalue (Transformation|GetActorLocation))
  ;[1 1 1] MonsterDeath
  (Components|SkeletalMesh|SetMorphTarget (Variables|Character|GetMesh) "Key 10" 1.0 true)
  (CallFunction|StopBlinking)
  (Effects|SpawnEmitteratLocation "/Game/Realistic_Starter_VFX_Pack_Vol2/Particles/Blood/P_Blood_Splat_Cone.P_Blood_Splat_Cone" (Transformation|GetActorLocation) "0, 0, 0" "2.500000,2.500000,2.500000")
  (Utilities|FlowControl|DoOnce false
    (:Completed
      (Variables|Default|SetMonsterDead? true)
      (Collision|SetCollisionEnabled (Variables|Default|GetCapsuleComponent) "NoCollision")
      (Development|PrintString "Embers")
      (Pawn|Components|CharacterMovement|SetMovementMode (Variables|Character|GetCharacterMovement) "MOVE_None" 0)
      (Rendering|SetVisibility (Variables|Default|GetBreath) false false)
      (Utilities|FlowControl|Delay 4.0)
      (Effects|SpawnEmitteratLocation "/Game/Realistic_Starter_VFX_Pack_Vol2/Particles/Sparks/P_Embers_A.P_Embers_A" (Math|Vector|MakeVector (.x _returnvalue) (.y _returnvalue) (- (.z _returnvalue) 2e+02)) "0, 0, 0" "0.500000,0.500000,0.500000")
      (Utilities|FlowControl|Delay 4.0)
      (Effects|SpawnEmitteratLocation "/Game/Realistic_Starter_VFX_Pack_Vol2/Particles/Fire/P_Fire_Big.P_Fire_Big" (Transformation|GetSocketLocation (Variables|Character|GetMesh) "spine_001") "0, 0, 0" "0.700000,0.700000,0.700000"))))

(event Custom|StopBlinking
  ;[1 1 1] Blinking Eyes Animation
  (bind _newtrack_0 (Timeline|Blinking Stop)
    (:Update
      (Components|SkeletalMesh|SetMorphTarget (Variables|Character|GetMesh) "Key 10" _newtrack_0 true))))

(event Custom|CheckPlayerNearby
  (bind _blackboardcomponent (Class|AIController|UseBlackboard (Variables|Default|GetAs%20AIController) "/Game/_Game/AI/BB_MonsterAI.BB_MonsterAI"))
  (if (ScalableFloat|GetValueasBool _blackboardcomponent (Utilities|Name|MakeLiteralName "CanSeePlayer"))
    (Variables|Default|SetAwareOfPlayer true)
    (else
      (Variables|Default|SetAwareOfPlayer false)))
  ;[1 1 1] CheckingDistanceToPlayer
  (if (Variables|Default|GetAwareOfPlayer)
    (if (< (Math|Vector|VectorLength (- (Transformation|GetWorldLocation (Variables|/Script/Engine.Character|GetMesh (Variables|Default|GetPlayer))) (Transformation|GetActorLocation))) 5e+02)
      (if (Variables|Default|GetPlayerCaught)
        (Variables|Default|SetAttacking false :!label _label)
        (else
          (Variables|Default|SetAttacking true)))
      (else
        (goto _label)))
    (else
      (Variables|Default|SetAttacking false))))

(event EventBeginPlay
  (bind _asaicontroller (Utilities|Casting|CastToAIController (Pawn|GetController)))
  ;[1 1 1] Blinking Eyes Animation
  (Variables|Default|SetAs%20AIController _asaicontroller)
  (bind _asbp_player_character (Utilities|Casting|CastToBP_PlayerCharacter (Game|GetPlayerCharacter 0)))
  (Variables|Default|SetPlayer _asbp_player_character)
  (Utilities|Time|SetTimerbyFunctionName 0 "CheckPlayerNearby" 0.1 true)
  (bind _newtrack_0 (Timeline|Blinking Play)
    (:Update
      (Components|SkeletalMesh|SetMorphTarget (Variables|Character|GetMesh) "Key 10" _newtrack_0 true))))

(event EventTick
  (params (DeltaSeconds :type Float%20%28single-precision%29)))

(fn ConstructionScript)