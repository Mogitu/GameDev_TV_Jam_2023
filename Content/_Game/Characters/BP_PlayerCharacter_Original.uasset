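; Player character Blueprint that handles the sequence of being caught by the monster.
; While Caught is set, Tick casts Monster to BP_MonsterCharacter and moves the player to its right-hand socket every frame.
; It also disables pawn control rotation on the camera and smoothly interpolates the view toward the monster's spine socket.
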(event EventBeginPlay)

(event Collision|EventActorBeginOverlap
  (params (OtherActor :type Actor%20Object%20Reference)))

(event EventTick
  (params (DeltaSeconds :type Float%20%28single-precision%29))
  (bind _cameracomponent (Variables|Default|GetCameraComponent))
  (if (Variables|Default|GetCaught)
    (bind _asbp_monster_character (Utilities|Casting|CastToBP_MonsterCharacter (Variables|Default|GetMonster)))
    (Transformation|SetActorLocation (Transformation|GetSocketLocation (Variables|/Script/Engine.Character|GetMesh _asbp_monster_character) "hand_RSocket") false false)
    (Variables|/Script/Engine.CameraComponent|SetbUsePawnControlRotation (Variables|Default|GetCameraComponent) false)
    (Transformation|SetWorldRotation _cameracomponent (Math|Interpolation|RInterpTo (Transformation|GetWorldRotation _cameracomponent) (Math|Rotator|FindLookatRotation (Transformation|GetActorLocation) (Transformation|GetSocketLocation (Variables|/Script/Engine.Character|GetMesh _asbp_monster_character) "spine_004Socket")) (Utilities|Time|GetWorldDeltaSeconds) 8.0) false false)))

(fn ConstructionScript)