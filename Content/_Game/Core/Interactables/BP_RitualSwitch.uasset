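; BP_RitualSwitch is an interactable switch that spawns the gun once all weapon parts are collected.
; On interact it asks GJGameMode whether every part is collected, then spawns BP_Gun at its SpawnPoint if the instigator is a GJPlayerCharacter.
; With parts missing it only prints a debug string.
; Its interact text is empty, and nothing here prevents repeat spawns.
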(event EventInteract
  (params (InstigatorPawn :type Pawn%20Object%20Reference))
  (bind _returnvalue (Game|GetGameMode))
  (bind (_asgjgame_mode _bsuccess) (Utilities|Casting|CastToGJGameMode _returnvalue))
  (if _bsuccess
    (bind _returnvalue_2 (Class|GJGameMode|AllWeaponPartsCollected _asgjgame_mode))
    (if _returnvalue_2
      (Utilities|Casting|CastToGJPlayerCharacter InstigatorPawn)
      (Game|SpawnActorfromClass "/Game/_Game/Weapon/BP_Gun.BP_Gun_C" (Transformation|GetWorldTransform (Variables|Default|GetSpawnPoint)) "AdjustIfPossibleButAlwaysSpawn" "MultiplyWithRoot" 0 0)
      (else
        (Development|PrintString "No bueno.")))))

(fn ConstructionScript)

(fn GetInteractText
  (params (InstigatorPawn :type Pawn%20Object%20Reference))
  (return ""))