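; BP_Door is an interactable door that swings open and closed when interacted with, offering an "Open Door" prompt.
; Each Interact plays an attached sound, flips the Opened flag and plays or reverses a Timeline.
; Timeline updates feed HandleDoor, which lerps the carved door mesh's yaw and disables its collision, with no re-enable in the graph.
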(event EventInteract
  (params (InstigatorPawn :type Pawn%20Object%20Reference))
  (Audio|SpawnSoundAttached "/Game/_Game/Audio/Door_Opening_1.Door_Opening_1" (Variables|Transformation|GetRootComponent) "None" "0, 0, 0" "0, 0, 0" "KeepRelativeOffset" false 5.0 1.0 0.0 0 0)
  (if (Variables|Default|GetOpened)
    (Variables|Default|SetOpened false)
    (bind _alpha (Timeline|Timeline Reverse)
      (:Update
        (CallFunction|HandleDoor _alpha)
        (Collision|SetCollisionEnabled (Variables|Default|GetSM_DoorCarved) "NoCollision")))
    (else
      (Variables|Default|SetOpened true)
      (Timeline|Timeline Play))))

(fn ConstructionScript)

(fn HandleDoor
  (params (Alpha :type Float%20%28double-precision%29))
  (Transformation|SetRelativeRotation (Variables|Default|GetSM_DoorCarved) (Math|Rotator|MakeRotator 0.0 0.0 (Math|Float|Lerp 0.0 1.3e+02 Alpha)) false false))

(fn GetInteractText
  (params (InstigatorPawn :type Pawn%20Object%20Reference))
  (return "Open Door"))